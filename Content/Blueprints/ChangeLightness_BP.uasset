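; ChangeLightness_BP is an actor that makes a static mesh blink between bright and dim through a material parameter.
; The construction script assigns a configurable mesh and creates a dynamic material instance from a source material on its first slot.
; At BeginPlay, a looping one-second timer drives a FlipFlop that alternates the Lightness scalar between a high and low value on the mesh's materials.
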(event `self.ReceiveBeginPlay`
  (`KismetSystemLibrary.K2_SetTimerDelegate` (delegate `Change Lightness`) 1.0 true))

(event `Change Lightness`
  (bind _staticmesh (`self.StaticMesh`))
  (`/Engine/EditorBlueprintResources/StandardMacros.FlipFlop`
    (:`A`
      (`MeshComponent.SetScalarParameterValueOnMaterials` _staticmesh "Lightness" 100.0))
    (:`B`
      (`MeshComponent.SetScalarParameterValueOnMaterials` _staticmesh "Lightness" 10.0))))

(fn `UserConstructionScript`
  (`StaticMeshComponent.SetStaticMesh` (`self.StaticMesh`) (`self.Source Mesh`))
  (bind _returnvalue (`PrimitiveComponent.CreateDynamicMaterialInstance` (`self.StaticMesh`) 0 (`self.Source Material`) "None"))
  (set `self.Dynamic Material Instance` _returnvalue))