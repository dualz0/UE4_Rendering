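; ChangeMaterial_BP is an actor Blueprint that alternates the material on its static mesh between grass and gold once per second.
; The construction script assigns the source mesh and a metal gold material to the first slot.
; On BeginPlay, a looping timer calls the ChangeMaterial event, where a FlipFlop switches that slot between the grass and gold materials, starting with grass.
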(event `self.ReceiveBeginPlay`
  (`KismetSystemLibrary.K2_SetTimerDelegate` (delegate `Change Material`) 1.0 true))

(event `Change Material`
  (bind _staticmesh (`self.StaticMesh`))
  (`/Engine/EditorBlueprintResources/StandardMacros.FlipFlop`
    (:`A`
      (`PrimitiveComponent.SetMaterial` _staticmesh 0 (`self.Material_Grass`)))
    (:`B`
      (`PrimitiveComponent.SetMaterial` _staticmesh 0 (`self.Material Gold`)))))

(fn `UserConstructionScript`
  (bind _staticmesh (`self.StaticMesh`))
  (`StaticMeshComponent.SetStaticMesh` _staticmesh (`self.Source Mesh`))
  (`PrimitiveComponent.SetMaterial` _staticmesh 0 "/Game/StarterContent/Materials/M_Metal_Gold.M_Metal_Gold"))