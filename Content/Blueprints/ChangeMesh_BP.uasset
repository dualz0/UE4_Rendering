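; ChangeMesh_BP is an actor that swaps its static mesh back and forth between two meshes on a timer.
; The construction script sets the source mesh, and BeginPlay starts a looping one-second timer.
; Each timer tick runs a FlipFlop that alternates between the new mesh and the source mesh.
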(event `self.ReceiveBeginPlay`
  (`KismetSystemLibrary.K2_SetTimerDelegate` (delegate `Change Mesh`) 1.0 true))

(event `Change Mesh`
  (bind _staticmesh (`self.StaticMesh`))
  (`/Engine/EditorBlueprintResources/StandardMacros.FlipFlop`
    (:`A`
      (`StaticMeshComponent.SetStaticMesh` _staticmesh (`self.New Mesh`)))
    (:`B`
      (`StaticMeshComponent.SetStaticMesh` _staticmesh (`self.Source Mesh`)))))

(fn `UserConstructionScript`
  (`StaticMeshComponent.SetStaticMesh` (`self.StaticMesh`) (`self.Source Mesh`)))