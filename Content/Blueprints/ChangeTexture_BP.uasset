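; Actor Blueprint that alternates a static mesh's texture between wood and grass at runtime.
; The construction script assigns the source mesh and creates a dynamic material instance from the source material on its first element.
; On BeginPlay, a looping one-second timer fires a FlipFlop that sets the instance's "Texture" parameter to one texture, then the other.
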(event `self.ReceiveBeginPlay`
  (`KismetSystemLibrary.K2_SetTimerDelegate` (delegate `Change Texture`) 1.0 true))

(event `Change Texture`
  (bind _dynamic_material_instance (`self.Dynamic Material Instance`))
  (`/Engine/EditorBlueprintResources/StandardMacros.FlipFlop`
    (:`A`
      (`MaterialInstanceDynamic.SetTextureParameterValue` _dynamic_material_instance "Texture" (`self.Texture Wood`)))
    (:`B`
      (`MaterialInstanceDynamic.SetTextureParameterValue` _dynamic_material_instance "Texture" (`self.Texture Grass`)))))

(fn `UserConstructionScript`
  (`StaticMeshComponent.SetStaticMesh` (`self.StaticMesh`) (`self.Source Mesh`))
  (bind _returnvalue (`PrimitiveComponent.CreateDynamicMaterialInstance` (`self.StaticMesh`) 0 (`self.Source Material`) "None"))
  (set `self.Dynamic Material Instance` _returnvalue))