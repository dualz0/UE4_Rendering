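; ChangeColor_BP is an actor that blinks its static mesh between yellow and black once per second.
; The construction script applies a configurable source mesh and creates a dynamic material instance from a source material on slot 0.
; BeginPlay starts a looping timer whose event uses a FlipFlop to alternately set the BaseColor vector parameter on the mesh's materials.
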(event `self.ReceiveBeginPlay`
  (`KismetSystemLibrary.K2_SetTimerDelegate` (delegate `Change Color`) 1.0 true))

(event `Change Color`
  (bind _staticmesh (`self.StaticMesh`))
  (`/Engine/EditorBlueprintResources/StandardMacros.FlipFlop`
    (:`A`
      (`MeshComponent.SetVectorParameterValueOnMaterials` _staticmesh "BaseColor" (1.0 1.0 0.0)))
    (:`B`
      (`MeshComponent.SetVectorParameterValueOnMaterials` _staticmesh "BaseColor" (0.0 0.0 0.0)))))

(fn `UserConstructionScript`
  (`StaticMeshComponent.SetStaticMesh` (`self.StaticMesh`) (`self.Source Mesh`))
  (bind _returnvalue (`PrimitiveComponent.CreateDynamicMaterialInstance` (`self.StaticMesh`) 0 (`self.Source Material`) "None"))
  (set `self.Dynamic Material Instance` _returnvalue))